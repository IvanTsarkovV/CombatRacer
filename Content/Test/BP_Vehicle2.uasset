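; BP_Vehicle2 is a test physics-driven vehicle that flies along its mesh's forward vector, with throttle, yaw and pitch input.
; Throttle axes step a clamped throttle value after a short delay and print it.
; Steering axes add torque around the mesh's up and right vectors.
; Tick counters spin with opposing torque, applies a constant downward force, and blends linear velocity toward forward direction scaled by throttle.
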(event EventBeginPlay)

(event EventTick
  (params (DeltaSeconds :type Float%20%28single-precision%29))
  (bind _staticmesh (Variables|Default|GetStaticMesh))
  (Class|PrimitiveComponent|AddTorqueinDegrees (Variables|Default|GetStaticMesh) (/ (Math|Vector|NegateVector (Physics|GetPhysicsAngularVelocityinDegrees (Variables|Default|GetStaticMesh) "None")) 0.5) "None" true)
  (Physics|AddForce (Variables|Default|GetStaticMesh) "0.000000,0.000000,-1500.000000" "None" true)
  (bind _returnvalue (Physics|GetPhysicsLinearVelocity _staticmesh "None"))
  (Physics|SetPhysicsLinearVelocity (Variables|Default|GetStaticMesh) (Math|Vector|Lerp(Vector) _returnvalue (* (Math|Vector|GetForwardVector _staticmesh) (* (Variables|Default|GetThrottleCurrent) 2.5e+02)) 0.01) false "None"))

(event Input|AxisEvents|InputAxisThrottleUp
  (params (AxisValue :type Float%20%28single-precision%29))
  (if (!= AxisValue 0.0)
    (Utilities|FlowControl|Delay 0.2)
    (bind _output_get (Variables|Default|SetThrottleCurrent (Math|Float|Clamp(Float) (+ (* AxisValue (Variables|Default|GetThrottleStep)) (Variables|Default|GetThrottleCurrent)) (Variables|Default|GetThrottleMin) (Variables|Default|GetThrottleMax))))
    (Development|PrintString (Utilities|String|ToString(Float) _output_get))))

(event Input|AxisEvents|InputAxisThrottleDown
  (params (AxisValue :type Float%20%28single-precision%29))
  (if (!= AxisValue 0.0)
    (Utilities|FlowControl|Delay 0.2)
    (bind _output_get (Variables|Default|SetThrottleCurrent (Math|Float|Clamp(Float) (+ (* AxisValue (Variables|Default|GetThrottleStep)) (Variables|Default|GetThrottleCurrent)) (Variables|Default|GetThrottleMin) (Variables|Default|GetThrottleMax))))
    (Development|PrintString (Utilities|String|ToString(Float) _output_get))))

(event Input|AxisEvents|InputAxisRightLeft
  (params (AxisValue :type Float%20%28single-precision%29))
  (Class|PrimitiveComponent|AddTorqueinDegrees (Variables|Default|GetStaticMesh) (Math|Vector|Lerp(Vector) "0, 0, 0" (* (* AxisValue (Variables|Default|GetRotationSpeed)) (Math|Vector|GetUpVector (Variables|Default|GetStaticMesh))) 0.1) "None" true))

(event Input|AxisEvents|InputAxisUpDown
  (params (AxisValue :type Float%20%28single-precision%29))
  (Class|PrimitiveComponent|AddTorqueinDegrees (Variables|Default|GetStaticMesh) (Math|Vector|Lerp(Vector) "0, 0, 0" (* (* AxisValue (Variables|Default|GetRotationSpeed)) (Math|Vector|GetRightVector (Variables|Default|GetStaticMesh))) 0.1) "None" true))

(fn ConstructionScript)